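; BP_FireAnt is a fire ant bug that spots the exterminator and records where it was seen.
; Its PawnSensing component casts each seen pawn to BP_Exterminator and writes that pawn's location to the ExterminatorLocation blackboard key.
; A validity check prints a debug message for an invalid character.
; The file holds no movement or attack logic, and its default BeginPlay, overlap and Tick events are disabled.
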(event `self.PawnSensing.OnSeePawn`
  (params (Pawn :type "Pawn Object Reference"))
  (bind _asbp_exterminator (cast `/Game/TheExterminator/BP_Exterminator` Pawn))
  (`/Engine/EditorBlueprintResources/StandardMacros.IsValid` _asbp_exterminator
    (:`Is Valid`
      _)
    (:`Is Not Valid`
      (`KismetSystemLibrary.PrintString` "CharacterInvalid!!!!")))
  (`BlackboardComponent.SetValueAsVector` (`AIBlueprintHelperLibrary.GetBlackboard` self) "ExterminatorLocation" (`self.K2_GetActorLocation` _asbp_exterminator)))

(fn `UserConstructionScript`
  (`parent.UserConstructionScript`))