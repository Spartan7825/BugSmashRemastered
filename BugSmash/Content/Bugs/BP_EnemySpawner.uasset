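; Enemy spawner actor that spawns queued bug classes one at a time at its own transform.
; AddBugtoQueue appends a class and calls SpawnBug only if a BP_FireAnt already overlaps the spawner's Sphere.
; SpawnBug spawns and removes the first entry, then sets a short function-name timer on itself to work through the queue, returning false when it is empty.
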(fn `AddBugtoQueue`
  (params (BugClass :type "/Game/Bugs/BP_FireAnt Class Reference"))
  (`KismetArrayLibrary.Array_Add` (`self.BugQueue`) BugClass)
  (if (`KismetArrayLibrary.Array_IsValidIndex` (`PrimitiveComponent.GetOverlappingActors` (`self.Sphere`) "/Game/Bugs/BP_FireAnt.BP_FireAnt_C"))
    (`self.SpawnBug`)))

(fn `SpawnBug`
  (returns (Success :type Boolean))
  ;[1 1 1] check if anything in array, if not escape the function with return node
  (if (`KismetArrayLibrary.Array_IsValidIndex` (`self.BugQueue`))
    (`|SpawnActorFromClass` (`|GetArrayItem` (`self.BugQueue`)) (`self.GetTransform`) "Undefined" "MultiplyWithRoot" null null)
    (`KismetArrayLibrary.Array_Remove` (`self.BugQueue`))
    (`KismetSystemLibrary.K2_SetTimer` null "SpawnBug" 2.0)
    (return true)
    (else
      (return false))))

(fn `UserConstructionScript`)